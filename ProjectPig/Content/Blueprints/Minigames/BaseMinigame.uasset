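; Base minigame actor that renders its scene through a capture component into a texture for display.
; On BeginPlay it creates a square render target for MinigameCapture and feeds it to a dynamic material's RenderIn parameter.
; ClickProcess_Event turns a coordinate on that image into a debug-drawn object trace from the capture, rotated to its orientation.
; The trace result is unused and ReleaseProcess_Event is an empty stub.
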(event `self.ReceiveBeginPlay`
  (bind _returnvalue (`KismetRenderingLibrary.CreateRenderTarget2D` 900 900))
  (bind _output_get (set `SceneCaptureComponent2D.TextureTarget` _returnvalue (`self.MinigameCapture`)))
  (bind _output_get_2 (set `self.MinigameRender` _output_get))
  (bind _returnvalue_2 (`KismetMaterialLibrary.CreateDynamicMaterialInstance` "/Game/MaterialsAndTextures/MinigameDisplay.MinigameDisplay"))
  (bind _output_get_3 (set `self.MinigameTexture` _returnvalue_2))
  (`MaterialInstanceDynamic.SetTextureParameterValue` _output_get_3 "RenderIn" _output_get_2))

(event `ClickProcess_Event`
  (params (MouseCoordinateOnCapture :type "Vector2D Structure"))
  (bind _minigamecapture (`self.MinigameCapture`))
  (bind _returnvalue (`SceneComponent.K2_GetComponentLocation` _minigamecapture))
  (bind (_returnvalue_x _returnvalue_y) (`KismetMathLibrary.BreakVector2D` (- MouseCoordinateOnCapture (/ (900.0 -900.0) (2.0 2.0)))))
  (`KismetSystemLibrary.LineTraceSingleForObjects` :`Start` _returnvalue :`End` (+ _returnvalue (`KismetMathLibrary.GreaterGreater_VectorRotator` (`KismetMathLibrary.MakeVector` 300.0 _returnvalue_x _returnvalue_y) (`SceneComponent.K2_GetComponentRotation` _minigamecapture))) :`ObjectTypes` (`self.MinigameIObjectTypes`) :`DrawDebugType` "ForDuration" :`DrawTime` 10.0)
  (if true
    _))

(event `ReleaseProcess_Event`)

(fn `UserConstructionScript`)