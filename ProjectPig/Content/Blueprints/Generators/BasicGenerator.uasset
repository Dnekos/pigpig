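; Basic generator Blueprint that computes a generated amount as a LargeFloat and targets a Storage actor.
; On BeginPlay it finds a Storage actor in the level with GetActorOfClass and sets it as the target storage.
; Generate passes BaseGenVal through ModifyValue, which multiplies it by TempMod, then wraps the result in a LargeFloat with a zero exponent.
; Nothing in this graph calls Generate or sends its result to storage.
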(event `self.ReceiveBeginPlay`
  (bind _returnvalue (`GameplayStatics.GetActorOfClass` "/Script/ProjectPig.Storage"))
  (`self.SetTargetStorage` _returnvalue))

(fn `Generate`
  (returns (ReturnValue :type "LargeFloat Object Reference"))
  (bind _valueout (`self.ModifyValue` (`self.BaseGenVal`)))
  (return (`LargeFloat.makeLargeFloat` _valueout)))

(fn `ModifyValue`
  (params (ValueIn :type "Float (double-precision)"))
  (returns (ValueOut :type "Float (double-precision)"))
  (return (* ValueIn (`self.TempMod`))))

(fn `UserConstructionScript`)