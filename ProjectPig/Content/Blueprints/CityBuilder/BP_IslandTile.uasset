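; BP_IslandTile is a clickable island tile for the city builder, on which a generator can be built or destroyed.
; Clicking opens a WB_ConstructionWindow initialized with the tile, which can later remove it.
; BuildGenerator spends mud from TestStorage via large-float subtraction, spawns BasicGenerator as a child actor and shows a cone, but returns true even on failure.
; DestroyGenerator removes that component, clears BuiltOn and hides the cone; GetGenerator is empty.
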(event `self.ReceiveActorOnClicked`
  (params (ButtonPressed :type "Key Structure"))
  (`KismetSystemLibrary.PrintString` "I was clicked")
  (bind _returnvalue (`|CreateWidget` "/Game/UI/WB_ConstructionWindow.WB_ConstructionWindow_C"))
  (`UserWidget.AddToViewport` _returnvalue 0)
  (bind _output_get (set `self.BuildWidget` _returnvalue))
  (`/Game/UI/WB_ConstructionWindow.InitMe` _output_get self))

(fn `BuildGenerator`
  (returns (Success :type Boolean))
  (bind _returnvalue (`GameplayStatics.GetActorOfClass` "/Game/TestStorage.TestStorage_C"))
  (bind _returnvalue_2 (`Storage.SubtractLargeFloat` _returnvalue (`LargeFloat.makeLargeFloat` 10.0)))
  (if _returnvalue_2
    (bind _returnvalue_3 (`AddComponent|NODE_AddChildActorComponent-0`))
    (`ChildActorComponent.SetChildActorClass` _returnvalue_3 "/Game/Blueprints/Generators/BasicGenerator.BasicGenerator_C")
    (set `self.GeneratorRef` _returnvalue_3)
    (set `self.BuiltOn` true)
    (`KismetSystemLibrary.PrintString` "built generator")
    (`SceneComponent.SetVisibility` (`self.Cone`) true false)
    (return true)
    (else
      (`KismetSystemLibrary.PrintString` "Not enough mud")
      (return true))))

(fn `ClearMyWidgets`
  (`Widget.RemoveFromParent` (`self.BuildWidget`)))

(fn `DestroyGenerator`
  (`ActorComponent.K2_DestroyComponent` (`self.GeneratorRef`))
  (set `self.BuiltOn` false)
  (`KismetSystemLibrary.PrintString` "Generator Destroyed")
  (`SceneComponent.SetVisibility` (`self.Cone`) false false))

(fn `GetGenerator`
  (returns (Generator :type "/Game/Blueprints/Generators/BasicGenerator Object Reference"))
  (return null))

(fn `UserConstructionScript`)