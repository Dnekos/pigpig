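; BP_IslandTile is a clickable city-builder tile that toggles a generator on and off.
; Clicking it checks BuiltOn, then either spawns a BasicGenerator through a dynamically added Child Actor Component or destroys the stored component.
; Both paths update BuiltOn, show or hide the Cone to match and print debug messages.
; GetGenerator is an unfinished stub that does not return the stored reference.
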(event `self.ReceiveActorOnClicked`
  (params (ButtonPressed :type "Key Structure"))
  (`KismetSystemLibrary.PrintString` "I was clicked")
  (if (`self.BuiltOn`)
    (`self.DestroyGenerator`)
    (else
      (`self.BuildGenerator`))))

(fn `BuildGenerator`
  (bind _returnvalue (`AddComponent|NODE_AddChildActorComponent-0`))
  (`ChildActorComponent.SetChildActorClass` _returnvalue "/Game/Generators/BasicGenerator.BasicGenerator_C")
  (set `self.GeneratorRef` _returnvalue)
  (set `self.BuiltOn` true)
  (`KismetSystemLibrary.PrintString` "built generator")
  (`SceneComponent.SetVisibility` (`self.Cone`) true false))

(fn `DestroyGenerator`
  (`ActorComponent.K2_DestroyComponent` (`self.GeneratorRef`))
  (set `self.BuiltOn` false)
  (`KismetSystemLibrary.PrintString` "Generator Destroyed")
  (`SceneComponent.SetVisibility` (`self.Cone`) false false))

(fn `GetGenerator`
  (returns (Generator :type "/Game/Generators/BasicGenerator Object Reference"))
  (return null))

(fn `UserConstructionScript`)