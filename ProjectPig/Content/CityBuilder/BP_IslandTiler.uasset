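; BP_IslandTiler lays out a rectangular island of hex tiles for the city builder in its construction script.
; Nested width and height loops derive hex spacing from the TileMesh bounds, Scale and Offset, with a FlipFlop staggering alternate rows by half a tile.
; The Instanced flag selects instanced static meshes or BP_IslandTile child actors.
; Circular-island tile counting and runtime spawning are unfinished and never run.
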(event `self.ReceiveBeginPlay`)

(fn `CalculateNumTiles`
  (locals (`Radius Remaining` :type Integer))
  (set `self.TilestoGenerate` 1)
  (bind _output_get (set `local.Radius Remaining` (`self.IslandRadius`)))
  (while (> _output_get 0)
    (set `self.TilestoGenerate` (+ (`self.TilestoGenerate`) (* (`local.Radius Remaining`) 6)))
    (set `local.Radius Remaining` (- (`local.Radius Remaining`) 1)))
  (return))

(fn `UserConstructionScript`
  (bind _returnvalue (`StaticMesh.GetBoundingBox` (`self.TileMesh`)))
  (`StaticMeshComponent.SetStaticMesh` (`self.InstancedStaticMesh`) (`self.TileMesh`))
  (if (`.IsValid` (break `Box` _returnvalue))
    (set `self.Radius` (* (.x (`.Max` (break `Box` _returnvalue))) (`self.Scale`)))
    (for _index (range 1 (+ (`self.IslandHeight`) 1))
      (for _index_2 (range 1 (+ (`self.IslandWidth`) 1))
        (if (`self.Instanced?`)
          (bind _returnvalue_2 (+ (* _index_2 (`self.Radius`) 1.0) (* _index_2 (`self.Offset`)) (`self.RowOffset`)))
          (bind _returnvalue_3 (+ (* (/ (* (`self.Radius`) 2.0) (`KismetMathLibrary.Sqrt` 3.0)) 0.75 _index) (* _index (`self.Offset`))))
          (`InstancedStaticMeshComponent.AddInstance` (`self.InstancedStaticMesh`) (`KismetMathLibrary.MakeTransform` (`KismetMathLibrary.MakeVector` _returnvalue_2 _returnvalue_3) (struct) (`KismetMathLibrary.Conv_DoubleToVector` (`self.Scale`))) false)
          (else
            (bind _returnvalue_4 (`AddComponent|NODE_AddChildActorComponent-0` :`RelativeTransform` (`KismetMathLibrary.MakeTransform` (`KismetMathLibrary.MakeVector` _returnvalue_2 _returnvalue_3) (struct) (`KismetMathLibrary.Conv_DoubleToVector` (`self.Scale`)))))
            (`ChildActorComponent.SetChildActorClass` _returnvalue_4 "/Game/CityBuilder/BP_IslandTile.BP_IslandTile_C"))))
      (`/Engine/EditorBlueprintResources/StandardMacros.FlipFlop`
        (:`A`
          (set `self.RowOffset` (* (`self.Radius`) -0.5)))
        (:`B`
          (set `self.RowOffset` 0.0))))
    (else
      (`KismetSystemLibrary.PrintString` "No Valid Tile Mesh for Island Tiler"))))