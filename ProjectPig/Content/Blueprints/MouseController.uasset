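; MouseController is a controller that moves its controlled pawn and shows the WB_MinigameMount minigame widget, created and added to the viewport on BeginPlay.
; Each Tick offsets the pawn in world X/Y from the side and forward axes, scaled by delta time, without sweeping for collision.
; The scale names are crossed: side input uses ForwardMovementScale and forward input uses SideMovementScale.
; Widget removal logic exists but is unconnected, so it never runs.
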(event `self.ReceiveBeginPlay`
  (bind _returnvalue (`|CreateWidget` "/Game/UI/WB_MinigameMount.WB_MinigameMount_C"))
  (bind _output_get (set `self.MinigameWidget` _returnvalue))
  (`UserWidget.AddToViewport` _output_get 0))

(event `self.ReceiveTick`
  (params (DeltaSeconds :type "Float (single-precision)"))
  (bind _returnvalue (`self.K2_GetPawn`))
  (`self.K2_SetActorLocation` _returnvalue (+ (`self.K2_GetActorLocation` _returnvalue) (`KismetMathLibrary.MakeVector` (* (`self.GetInputAxisValue`) DeltaSeconds (`self.ForwardMovementScale`)) (* (`self.GetInputAxisValue`) DeltaSeconds (`self.SideMovementScale`)) (* 0.0 DeltaSeconds))) false false))

(event `Key|E`
  (params (Key :type "Key Structure")))

(fn `UserConstructionScript`)